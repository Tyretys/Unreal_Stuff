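; Locker hiding spot that lets the player toggle hiding from AI sight with an interact input.
; Box overlap caches the character and gates input to when they are nearby.
; Interact swings the door via a timeline and toggles mesh, collision, movement and sight stimulus, blending the camera between locker and player.
; A short delay then re-enables input and reopens the gate, so interaction survives the collision change.
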(event OnComponentBeginOverlap(Box)
  (params (OverlappedComponent :type Primitive%20Component%20Object%20Reference) (OtherActor :type Actor%20Object%20Reference) (OtherComp :type Primitive%20Component%20Object%20Reference) (OtherBodyIndex :type Integer) (bFromSweep :type Boolean) (SweepResult :type Hit%20Result%20Structure%20%28by%20ref%29))
  (bind _asbp_third_person_character (Utilities|Casting|CastToBP_ThirdPersonCharacter OtherActor))
  (Variables|Default|SetPlayer%20REFF _asbp_third_person_character)
  (Input|EnableInput (Game|GetPlayerController 0))
  (Utilities|FlowControl|Gate true) ; enters at Open
)

(event OnComponentEndOverlap(Box)
  (params (OverlappedComponent :type Primitive%20Component%20Object%20Reference) (OtherActor :type Actor%20Object%20Reference) (OtherComp :type Primitive%20Component%20Object%20Reference) (OtherBodyIndex :type Integer))
  (bind _returnvalue (Game|GetPlayerController 0))
  (Utilities|Casting|CastToBP_ThirdPersonCharacter OtherActor)
  (Input|DisableInput _returnvalue)
  (Utilities|FlowControl|Gate true) ; enters at Close
)

(event Custom|Animate%20Door
  (bind _dooropennig (Timeline|OpenLockerDoor PlayFromStart)
    (:Update
      (Transformation|SetRelativeRotation (Variables|Default|GetLocker_Door) (Math|Rotator|MakeRotator 0.0 0.0 (Math|Float|Lerp (Variables|Default|GetCloseAngle) (Variables|Default|GetOpenAngle) _dooropennig)) false false))))

(event EventInteract
  (Utilities|FlowControl|Gate true :!label _label
    (:Exit
      (Utilities|FlowControl|Sequence
        (:then_0
          (CallFunction|HidePlayer)
          (Utilities|FlowControl|Delay 0.2)
          (Input|EnableInput (Game|GetPlayerController 0))
          (goto _label Open))
        (:then_1
          (CallFunction|AnimateDoor))))))

(fn ConstructionScript)

(fn HidePlayer
  (bind _returnvalue (Game|GetPlayerController 0))
  (bind _player_reff (Variables|Default|GetPlayer%20REFF))
  (bind _player_reff_2 (Variables|Default|GetPlayer%20REFF))
  (bind _mesh (Variables|/Script/Engine.Character|GetMesh _player_reff))
  (bind _aiperceptionstimulisource (Variables|/Game/ThirdPerson/Blueprints/BP_ThirdPersonCharacter.BP_ThirdPersonCharacter_C|GetAIPerceptionStimuliSource _player_reff_2))
  (if (Variables|Default|GetIsHiding?)
    (Variables|Default|SetIsHiding? false)
    (Variables|/Game/ThirdPerson/Blueprints/BP_ThirdPersonCharacter.BP_ThirdPersonCharacter_C|SetCanMove? _player_reff true)
    (Rendering|SetVisibility _mesh true false)
    (Collision|SetActorEnableCollision _player_reff true)
    (Game|Player|SetViewTargetwithBlend _returnvalue _player_reff 0.6 "VTBlend_Linear" 0.0 false)
    (Class|AIPerceptionStimuliSourceComponent|RegisterforSense _aiperceptionstimulisource "/Script/AIModule.AISense_Sight")
    (else
      (Variables|Default|SetIsHiding? true)
      (Variables|/Game/ThirdPerson/Blueprints/BP_ThirdPersonCharacter.BP_ThirdPersonCharacter_C|SetCanMove? _player_reff false)
      (Rendering|SetVisibility _mesh false false)
      (Collision|SetActorEnableCollision _player_reff false)
      (Game|Player|SetViewTargetwithBlend _returnvalue self 0.6 "VTBlend_Linear" 0.0 false)
      (Class|AIPerceptionStimuliSourceComponent|UnregisterfromSense _aiperceptionstimulisource "/Script/AIModule.AISense_Sight"))))