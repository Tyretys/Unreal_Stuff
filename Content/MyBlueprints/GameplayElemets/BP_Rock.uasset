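; BP_Rock is a small projectile rock that makes a noise where it lands, which AI hearing can detect.
; On BeginPlay it passes its Velocity variable to the ProjectileMovement component, and the construction script scales the mesh down.
; The first mesh hit, gated by DoOnce, reports an AI noise event at the rock's location, prints a debug string and plays the hit sound.
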(event OnComponentHit(StaticMesh)
  (params (HitComponent :type Primitive%20Component%20Object%20Reference) (OtherActor :type Actor%20Object%20Reference) (OtherComp :type Primitive%20Component%20Object%20Reference) (NormalImpulse :type Vector :default "0, 0, 0") (Hit :type Hit%20Result%20Structure%20%28by%20ref%29))
  (Utilities|FlowControl|DoOnce false
    (:Completed
      (Class|AISenseHearing|ReportNoiseEvent (Transformation|GetActorLocation) 0.7 self 0.0 "")
      (Development|PrintString "Hit")
      (Audio|PlaySoundatLocation "/Game/MyBlueprints/VFX/hit_sound.hit_sound" (Transformation|GetActorLocation) "0, 0, 0" 1.0 1.0 0.0 0 0 0 0))))

(event EventBeginPlay
  (Variables|/Script/Engine.MovementComponent|SetVelocity (Variables|Default|GetProjectileMovement) (Variables|Default|GetVelocity)))

(fn ConstructionScript
  (Transformation|SetWorldScale3D (Variables|Default|GetStaticMesh) "0.100000,0.100000,0.100000"))